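; Destructible mesh actor for DogFight that loses health from any damage and is destroyed at zero.
; On BeginPlay the authority derives health from summed mesh world scale times a modifier unless preset, and sets mass scale from the same size formula.
; Damage is handled on the authority, which passes the health ratio through a Replicate event to the HealthRatio material parameter, using a dynamic material instance created at start.
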(event `self.ReceiveBeginPlay`
  (bind (_returnvalue_x _returnvalue_y _returnvalue_z) (`KismetMathLibrary.BreakVector` (`SceneComponent.K2_GetComponentScale` (`self.StaticMeshComponent`))))
  (bind _returnvalue (* (`self.ScaleHealthModifier`) (+ _returnvalue_x _returnvalue_y _returnvalue_z)))
  (`self.Replicate_CreateInstance`)
  (`/Engine/EditorBlueprintResources/ActorMacros.Switch Has Authority`
    (:`Authority`
      ;[1 1 1] If health has not been manually set
      (if (< (`self.Health`) 0.0)
        (set `self.Health` _returnvalue))
      (set `self.MaxHealth` (`self.Health`))
      (`PrimitiveComponent.SetMassScale` (`self.StaticMeshComponent`) "None" (* 1000 _returnvalue)))))

(event `Replicate_CreateInstance`
  (bind _returnvalue (`KismetMaterialLibrary.CreateDynamicMaterialInstance` (`PrimitiveComponent.GetMaterial` (`self.StaticMeshComponent`) 0)))
  (`PrimitiveComponent.SetMaterial` (`self.StaticMeshComponent`) 0 _returnvalue))

(event `self.ReceiveAnyDamage`
  (params (Damage :type "Float (single-precision)") (DamageType :type "DamageType Object Reference") (InstigatedBy :type "Controller Object Reference") (DamageCauser :type "Actor Object Reference"))
  (`/Engine/EditorBlueprintResources/ActorMacros.Switch Has Authority`
    (:`Authority`
      (set `self.Health` (- (`self.Health`) Damage))
      (`self.Replicate_SetMaterialColor` (/ (`self.Health`) (`self.MaxHealth`)))
      (if (<= (`self.Health`) 0.0)
        (`self.K2_DestroyActor`)))))

(event `Replicate_SetMaterialColor`
  (params (ParameterValue :type "Float (double-precision)"))
  (`MeshComponent.SetScalarParameterValueOnMaterials` (`self.StaticMeshComponent`) "HealthRatio" ParameterValue))

(fn `UserConstructionScript`)